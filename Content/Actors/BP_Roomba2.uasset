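; Playable or AI-possessed Roomba pawn for a balloon-popping fight, with a knife and three balloons, which turn red under non-player control.
; Input either turns or drives it forward, with forward movement setting the looping vacuum sound's volume.
; Knife overlaps with tagged balloons call PopBalloon on the owning Roomba.
; Unless invulnerable, it hides the balloon, decrements its count, plays effects and camera shake, and notifies GM_RoombaFightClub.
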(event `InputAction|Exit`
  (params (Key :type "Key Structure" :default "AnyKey"))
  (:`Pressed`
    (`KismetSystemLibrary.QuitGame` null "Quit")))

(event `InputAction|Test`
  (params (Key :type "Key Structure" :default "AnyKey")))

(event `self.ReceivePossessed`
  (params (NewController :type "Controller Object Reference"))
  (if (not (`Controller.IsPlayerController` NewController))
    (`self.SetRedBaloons`)))

(event `self.ReceiveBeginPlay`
  (bind _returnvalue (`GameplayStatics.SpawnSoundAttached` "/Game/Sounds/Effects/Vacuum_Looped_Cue.Vacuum_Looped_Cue" (`self.Roomba`) "None" (0.0 0.0 0.0) (struct) "SnapToTarget" false 0.0))
  (set `self.VacuumSound` _returnvalue))

(event `InputAxis|TurnRight_P1`
  (params (AxisValue :type "Float (single-precision)"))
  (`self.AddControllerYawInput` (* AxisValue 1.0)))

(event `InputAxis|MoveForward_P1`
  (params (AxisValue :type "Float (single-precision)"))
  (bind _returnvalue (* (`self.GetActorForwardVector`) AxisValue))
  (if (== (`self.GetInputAxisValue`) 0.0)
    (`self.AddMovementInput` _returnvalue)
    (`AudioComponent.SetVolumeMultiplier` (`self.VacuumSound`) (`KismetMathLibrary.VSize` _returnvalue))))

(event `self.Knife.OnComponentBeginOverlap`
  (params (OverlappedComponent :type "PrimitiveComponent Object Reference") (OtherActor :type "Actor Object Reference") (OtherComp :type "PrimitiveComponent Object Reference") (OtherBodyIndex :type Integer) (bFromSweep :type Boolean) (SweepResult :type "HitResult Structure (by ref)"))
  (if (`ActorComponent.ComponentHasTag` OtherComp "Balloon")
    (bind _asbp_roomba_2 (cast `/Game/Actors/BP_Roomba2` OtherActor))
    (`self.PopBalloon` _asbp_roomba_2 OtherComp)))

(event `InputAction|ScreenShot`
  (params (Key :type "Key Structure" :default "AnyKey"))
  (:`Pressed`
    (bind _returnvalue (`GameplayStatics.GetPlayerControllerID` null))
    (`KismetSystemLibrary.ExecuteConsoleCommand` "HighResShot 2" (`GameplayStatics.GetPlayerController` _returnvalue))))

(fn `PopBalloon`
  (params (Balloon :type "PrimitiveComponent Object Reference"))
  (bind _returnvalue (`SceneComponent.K2_GetComponentLocation` Balloon))
  (if (not (`self.Invul`))
    (`SceneComponent.SetVisibility` Balloon false false)
    (`PrimitiveComponent.SetCollisionEnabled` Balloon "NoCollision")
    (set `self.BalloonCount` (- (`self.BalloonCount`) 1))
    (bind _asgm_roomba_fight_club (cast `/Game/Logic/GM_RoombaFightClub` (`GameplayStatics.GetGameMode`)))
    (`GameplayStatics.PlaySoundAtLocation` "/Game/Sounds/Effects/Balloon_Cue.Balloon_Cue" _returnvalue)
    (`GameplayStatics.SpawnEmitterAttached` "/Game/Particles/PS_Confetti.PS_Confetti" Balloon "None" (0.0 0.0 0.0) (struct) "SnapToTarget")
    (`/Game/Logic/GM_RoombaFightClub.HandlePop` _asgm_roomba_fight_club)
    (`GameplayStatics.PlayWorldCameraShake` "/Game/Actors/BP_PopShake.BP_PopShake_C" _returnvalue 0.0 100000.0)))

(fn `SetRedBaloons`
  (`|ExecutionSequence`
    (:`then_0`
      (bind _returnvalue (`PrimitiveComponent.CreateDynamicMaterialInstance` (`self.Balloon`) 0 "/Game/Materials/Mat_Flex_Master.Mat_Flex_Master"))
      (`MaterialInstanceDynamic.SetVectorParameterValue` _returnvalue "BaseColor" (struct :`R` 1.0 :`A` 1.0)))
    (:`then_1`
      (bind _returnvalue_2 (`PrimitiveComponent.CreateDynamicMaterialInstance` (`self.Balloon2`) 0 "/Game/Materials/Mat_Flex_Master.Mat_Flex_Master"))
      (`MaterialInstanceDynamic.SetVectorParameterValue` _returnvalue_2 "BaseColor" (struct :`R` 1.0 :`A` 1.0)))
    (:`then_2`
      (bind _returnvalue_3 (`PrimitiveComponent.CreateDynamicMaterialInstance` (`self.Balloon3`) 0 "/Game/Materials/Mat_Flex_Master.Mat_Flex_Master"))
      (`MaterialInstanceDynamic.SetVectorParameterValue` _returnvalue_3 "BaseColor" (struct :`R` 1.0 :`A` 1.0)))))

(fn `UserConstructionScript`)