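; BP_Roomba is a player-one Roomba with a knife for popping balloons.
; Turn input rotates the actor directly, while forward input applies a physics force along its facing, only when turn input is zero.
; Knife hit and overlap events check for the Balloon tag but only print "pop".
; Balloon spawn-and-constrain logic is unconnected, and the TurnRight function is an empty stub.
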(event `InputAxis|TurnRight_P1`
  (params (AxisValue :type "Float (single-precision)"))
  (`self.K2_AddActorLocalRotation` (`KismetMathLibrary.MakeRotator` 0.0 0.0 (* AxisValue 5.0))))

(event `InputAxis|MoveForward_P1`
  (params (AxisValue :type "Float (single-precision)"))
  (if (== (`self.GetInputAxisValue`) 0.0)
    (`PrimitiveComponent.AddForce` (`self.BSP_Roomba`) (* (`self.GetActorForwardVector`) (* AxisValue (`self.ForwardThrust`))) "None" false)))

(event `self.ReceiveBeginPlay`)

(event `self.ReceiveTick`
  (params (DeltaSeconds :type "Float (single-precision)")))

(event `self.Knife.OnComponentHit`
  (params (HitComponent :type "PrimitiveComponent Object Reference") (OtherActor :type "Actor Object Reference") (OtherComp :type "PrimitiveComponent Object Reference") (NormalImpulse :type "Vector Structure") (Hit :type "HitResult Structure (by ref)"))
  (if (`ActorComponent.ComponentHasTag` OtherComp "Balloon")
    (`KismetSystemLibrary.PrintString` "pop")))

(event `self.Knife.OnComponentBeginOverlap`
  (params (OverlappedComponent :type "PrimitiveComponent Object Reference") (OtherActor :type "Actor Object Reference") (OtherComp :type "PrimitiveComponent Object Reference") (OtherBodyIndex :type Integer) (bFromSweep :type Boolean) (SweepResult :type "HitResult Structure (by ref)"))
  (if (`ActorComponent.ComponentHasTag` OtherComp "Balloon")
    (`KismetSystemLibrary.PrintString` "pop")))

(fn `TurnRight`
  (params (Direction :type "Float (double-precision)") (DeltaTime :type "Float (double-precision)")))

(fn `UserConstructionScript`)