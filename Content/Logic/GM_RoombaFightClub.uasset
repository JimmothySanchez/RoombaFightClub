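; Game mode for a Roomba balloon-popping fight, running the main menu, round setup and end screen.
; StartRound spawns roombas at unoccupied PlayerStarts, pitting Player 1 against a behavior-tree AI or second local player.
; HandlePop makes all roombas invulnerable and flags the round over if any has no balloons left.
; Tick then ramps slow motion and lowers music pitch before resetting positions and vulnerability, or showing the end screen.
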(event `self.ReceiveBeginPlay`
  (if false
    (`self.StartRound` (`self.PlayerCount`))
    (else
      (`self.LoadMainMenu`))))

(event `self.ReceiveTick`
  (params (DeltaSeconds :type "Float (single-precision)"))
  (bind _returnvalue (/ (`self.TimeSinceRound`) (`self.PostRoundLength`)))
  (if (`self.AfterHit`)
    (set `self.TimeSinceRound` (+ DeltaSeconds (`self.TimeSinceRound`)))
    (if (> (`self.TimeSinceRound`) (`self.PostRoundLength`))
      (set `self.TimeSinceRound` 0.0)
      (set `self.AfterHit` false)
      (`GameplayStatics.SetGlobalTimeDilation` 1.0)
      (`AudioComponent.SetPitchMultiplier` (`self.BackgroundMusic`) 1.0)
      (if (`self.RoundOver`)
        (`self.LoadEndScreen`)
        (else
          (`self.MovePlayersToStart`)))
      (else
        (`GameplayStatics.SetGlobalTimeDilation` (`KismetMathLibrary.Lerp` 0.3 0.1 _returnvalue))
        (`AudioComponent.SetPitchMultiplier` (`self.BackgroundMusic`) (`KismetMathLibrary.Lerp` 1.0 0.25 _returnvalue))))))

(fn `GetEmptySpawnLocation`
  (returns (Location :type "Vector Structure") (Rotation :type "Rotator Structure"))
  (bind _outactors (`GameplayStatics.GetAllActorsOfClass` "/Script/Engine.PlayerStart"))
  (for _array_element _outactors
    (bind _returnvalue (`self.K2_GetActorLocation` _array_element))
    (bind (_outhit _returnvalue_2) (`KismetSystemLibrary.SphereTraceSingleForObjects` _returnvalue (0.0 0.0 0.0) 150.0 (`|MakeArray` "ObjectTypeQuery3" :!type "EObjectTypeQuery Enum")))
    (if (not _returnvalue_2)
      (return _returnvalue (`self.K2_GetActorRotation` _array_element)))))

(fn `GetMenuCamera`
  (returns (MenuCam :type "CameraActor Object Reference"))
  (bind _outactors (`GameplayStatics.GetAllActorsWithTag` "MenuCam"))
  (bind _ascamera_actor (cast `CameraActor` (`KismetArrayLibrary.Array_Get` _outactors)))
  (return _ascamera_actor))

(fn `HandlePop`
  (`|ExecutionSequence`
    (:`then_0`
      (bind _outactors (`GameplayStatics.GetAllActorsOfClass` "/Game/Actors/BP_Roomba2.BP_Roomba2_C"))
      (for _array_element _outactors
        (set `/Game/Actors/BP_Roomba2.Invul` true _array_element)
        (if (== (`/Game/Actors/BP_Roomba2.BalloonCount` _array_element) 0)
          (set `self.RoundOver` true))))
    (:`then_1`
      (set `self.AfterHit` true))))

(fn `LoadEndScreen`
  (bind _returnvalue (`GameplayStatics.GetPlayerController` 0))
  (`|ExecutionSequence`
    (:`then_0`
      (bind _returnvalue_2 (`|CreateWidget` "/Game/UI/Widget_EndScreen.Widget_EndScreen_C" _returnvalue))
      (`UserWidget.AddToViewport` _returnvalue_2 0)
      (`WidgetBlueprintLibrary.SetInputMode_UIOnlyEx` _returnvalue _returnvalue_2 "LockAlways")
      (set `PlayerController.bShowMouseCursor` true _returnvalue))
    (:`then_1`
      (bind _menucam (`self.GetMenuCamera`))
      (`PlayerController.SetViewTargetWithBlend` _returnvalue _menucam 0.01 "VTBlend_Linear" 0.0 true)
      (`AudioComponent.Stop` (`self.BackgroundMusic`)))
    (:`then_2`
      (bind _asplayer_controller (cast `PlayerController` (`self.P2`)))
      (`GameplayStatics.RemovePlayer` _asplayer_controller))))

(fn `LoadMainMenu`
  (bind _returnvalue (`GameplayStatics.GetPlayerController` 0))
  (`|ExecutionSequence`
    (:`then_0`
      (bind _returnvalue_2 (`|CreateWidget` "/Game/UI/Widget_MainMenu.Widget_MainMenu_C" _returnvalue))
      (`UserWidget.AddToViewport` _returnvalue_2 0)
      (`WidgetBlueprintLibrary.SetInputMode_UIOnlyEx` _returnvalue _returnvalue_2 "LockAlways")
      (set `PlayerController.bShowMouseCursor` true _returnvalue))
    (:`then_1`
      (bind _menucam (`self.GetMenuCamera`))
      (`PlayerController.SetViewTargetWithBlend` _returnvalue _menucam 0.01 "VTBlend_Linear" 0.0 true))))

(fn `MovePlayersToStart`
  (bind _outactors (`GameplayStatics.GetAllActorsOfClass` "/Game/Actors/BP_Roomba2.BP_Roomba2_C"))
  (for _array_element _outactors
    (bind (_location _rotation) (`self.GetEmptySpawnLocation`))
    (`self.K2_TeleportTo` _array_element _location _rotation)
    (set `/Game/Actors/BP_Roomba2.Invul` false _array_element)))

(fn `StartRound`
  (params (InPlayerCount :type Integer))
  (bind _returnvalue (`GameplayStatics.GetPlayerController` 0))
  (bind _returnvalue_2 (`GameplayStatics.SpawnSoundAtLocation` "/Game/Sounds/Music/InGameMusic_Cue.InGameMusic_Cue"))
  (set `self.BackgroundMusic` _returnvalue_2)
  (set `self.PlayerCount` InPlayerCount)
  (`WidgetBlueprintLibrary.SetInputMode_GameOnly` _returnvalue)
  (set `PlayerController.bShowMouseCursor` false _returnvalue)
  (bind (_location _rotation) (`self.GetEmptySpawnLocation`))
  (bind _returnvalue_3 (`|SpawnActorFromClass` "/Game/Actors/BP_Roomba2.BP_Roomba2_C" (`KismetMathLibrary.MakeTransform` _location _rotation) "Undefined" "OverrideRootScale"))
  (`Controller.Possess` _returnvalue _returnvalue_3)
  (set `/Game/Actors/BP_Roomba2.PlayerName` "Player 1" _returnvalue_3)
  (switch `int` (`self.PlayerCount`)
    (:`1`
      (bind (_location_2 _rotation_2) (`self.GetEmptySpawnLocation`))
      (bind _returnvalue_4 (`AIBlueprintHelperLibrary.SpawnAIFromClass` "/Game/Actors/BP_Roomba2.BP_Roomba2_C" "/Game/Logic/AI/BT_Roomba.BT_Roomba" _location_2 _rotation_2))
      (bind _asbp_roomba_2 (cast `/Game/Actors/BP_Roomba2` _returnvalue_4))
      (set `/Game/Actors/BP_Roomba2.PlayerName` "Computer" _asbp_roomba_2))
    (:`2`
      (bind _returnvalue_5 (`GameplayStatics.CreatePlayer` -1))
      (set `self.P2` _returnvalue_5)
      (`WidgetBlueprintLibrary.SetInputMode_GameOnly` _returnvalue_5)
      (set `PlayerController.bShowMouseCursor` false _returnvalue_5)
      (bind (_location_3 _rotation_3) (`self.GetEmptySpawnLocation`))
      (bind _returnvalue_6 (`|SpawnActorFromClass` "/Game/Actors/BP_Roomba2.BP_Roomba2_C" (`KismetMathLibrary.MakeTransform` _location_3 _rotation_3) "Undefined" "OverrideRootScale"))
      (`Controller.Possess` _returnvalue_5 _returnvalue_6)
      (set `/Game/Actors/BP_Roomba2.PlayerName` "Player 2" _returnvalue_6)
      (`/Game/Actors/BP_Roomba2.SetRedBaloons` _returnvalue_6))))

(fn `UserConstructionScript`)